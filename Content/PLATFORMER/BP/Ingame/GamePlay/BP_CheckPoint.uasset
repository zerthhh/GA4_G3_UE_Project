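; Checkpoint actor for the platformer that records itself as the respawn reference when the player character enters its trigger box.
; On overlap by BP_ThirdPersonCharacter, it sets itself as LastCheckPoint on GM_Platformer, swaps the unchecked mesh for the checked one and plays the checkpoint sound.
; The construction script sizes the trigger box from the TriggerBoxSize variable.
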(event OnComponentBeginOverlap(TB_Checkpoint)
  (params (OverlappedComponent :type Primitive%20Component%20Object%20Reference) (OtherActor :type Actor%20Object%20Reference) (OtherComp :type Primitive%20Component%20Object%20Reference) (OtherBodyIndex :type Integer) (bFromSweep :type Boolean) (SweepResult :type Hit%20Result%20Structure%20%28by%20ref%29))
  (Utilities|Casting|CastToBP_ThirdPersonCharacter OtherActor)
  (bind _asgm_platformer (Utilities|Casting|CastToGM_Platformer (Game|GetGameMode)))
  (Variables|/Game/PLATFORMER/BP/Ingame/GM/GM_Platformer.GM_Platformer_C|SetLastCheckPoint _asgm_platformer self)
  (Rendering|SetVisibility (Variables|Default|GetSM_CheckpointNoCheck) false false)
  (Rendering|SetVisibility (Variables|Default|GetSM_CheckpointCheck) true false)
  (Audio|PlaySound2D (Variables|/Game/PLATFORMER/DATA/PDA_GameInfo.PDA_GameInfo_C|GetCheckPointSFX (Variables|Default|GetGameInfos)) 1.0 1.0 0.0 0 0))

(fn ConstructionScript
  (Components|Box|SetBoxExtent (Variables|Default|GetTB_Checkpoint) (Variables|Default|GetTrigger%20Box%20Size) true))