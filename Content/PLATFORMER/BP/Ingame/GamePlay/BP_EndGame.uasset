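; BP_EndGame is the finish-line actor of the platformer, ending the level when the player character overlaps its TB_FinishLine trigger.
; On overlap it stops the GS_Platformer timer, derives the final time, and shows WBP_EndGame with the next level to open.
; It shows the mouse cursor, disables pawn input, sends score and time to GI_Platformer's EndGameCallback, and plays the win sound.
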(event OnComponentBeginOverlap(TB_FinishLine)
  (params (OverlappedComponent :type Primitive%20Component%20Object%20Reference) (OtherActor :type Actor%20Object%20Reference) (OtherComp :type Primitive%20Component%20Object%20Reference) (OtherBodyIndex :type Integer) (bFromSweep :type Boolean) (SweepResult :type Hit%20Result%20Structure%20%28by%20ref%29))
  (bind _returnvalue (Game|GetPlayerController 0))
  (bind _asbp_third_person_character (Utilities|Casting|CastToBP_ThirdPersonCharacter (Game|GetPlayerCharacter 0)))
  (if (== OtherActor _asbp_third_person_character)
    (bind _asgs_platformer (Utilities|Casting|CastToGS_Platformer (Game|GetGameState)))
    (Utilities|Time|ClearandInvalidateTimerbyHandle (Variables|/Game/PLATFORMER/BP/Ingame/GM/GS_Platformer.GS_Platformer_C|GetTimer%20Reference _asgs_platformer))
    (Variables|Default|SetFinalTime (- (Variables|/Game/PLATFORMER/DATA/PDA_GameInfo.PDA_GameInfo_C|GetGameDuration (Variables|Default|GetGame%20Infos)) (Variables|/Game/PLATFORMER/BP/Ingame/GM/GS_Platformer.GS_Platformer_C|GetGame%20Duration _asgs_platformer)))
    (bind _returnvalue_2 (UserInterface|CreateWidget "/Game/PLATFORMER/BP/Ingame/UI/WBP_EndGame.WBP_EndGame_C" 0 0))
    (Variables|/Game/PLATFORMER/BP/Ingame/UI/WBP_EndGame.WBP_EndGame_C|SetLevelToOpen _returnvalue_2 (Variables|Default|GetLevel%20to%20Open))
    (UserInterface|Viewport|AddtoViewport _returnvalue_2 0)
    (Variables|/Script/Engine.PlayerController|SetbShowMouseCursor _returnvalue true)
    (Input|DisableInput 0)
    (Input|DisableInput (Pawn|GetControlledPawn _returnvalue) 0)
    (bind _asbp_third_person_character_2 (Utilities|Casting|CastToBP_ThirdPersonCharacter (Game|GetPlayerCharacter 0)))
    (bind _asgi_platformer (Utilities|Casting|CastToGI_Platformer (Game|GetGameInstance)))
    (Default|EndGameCallback _asgi_platformer (Variables|/Game/PLATFORMER/BP/Ingame/Player/BP_ThirdPersonCharacter.BP_ThirdPersonCharacter_C|GetCurrentScore _asbp_third_person_character_2) (Variables|Default|GetFinalTime))
    (Audio|PlaySound2D (Variables|/Game/PLATFORMER/DATA/PDA_GameInfo.PDA_GameInfo_C|GetWinSFX (Variables|Default|GetGame%20Infos)) 1.0 1.0 0.0 0 0)))

(event EventBeginPlay)

(event Collision|EventActorBeginOverlap
  (params (OtherActor :type Actor%20Object%20Reference)))

(event EventTick
  (params (DeltaSeconds :type Float%20%28single-precision%29)))

(fn ConstructionScript)