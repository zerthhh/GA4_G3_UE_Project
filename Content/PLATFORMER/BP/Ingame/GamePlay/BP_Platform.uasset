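; Moving platform actor that can optionally wobble and fall when the player character steps on it.
; A movement timeline, started at BeginPlay with a configurable play rate, lerps the mesh toward an end location.
; Trigger overlap stops that motion and chains a wobble timeline into a falling timeline offset from the current position.
; After a delay, the fall reverses, rotation resets, and normal movement resumes.
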(event OnComponentBeginOverlap(TB_PlatformFalling)
  (params (OverlappedComponent :type Primitive%20Component%20Object%20Reference) (OtherActor :type Actor%20Object%20Reference) (OtherComp :type Primitive%20Component%20Object%20Reference) (OtherBodyIndex :type Integer) (bFromSweep :type Boolean) (SweepResult :type Hit%20Result%20Structure%20%28by%20ref%29))
  (if (Variables|Default|GetEnable%20Platform%20Falling)
    (bind _asbp_third_person_character (Utilities|Casting|CastToBP_ThirdPersonCharacter (Game|GetPlayerCharacter 0)))
    (if (== OtherActor _asbp_third_person_character)
      (Audio|Components|Audio|Stop (Variables|Default|GetTL_PlatformMovement))
      (Variables|Default|SetPlatform%20Current%20Rotation (Variables|/Script/Engine.SceneComponent|GetRelativeRotation (Variables|Default|GetSM_PlatformFalling)))
      (CallFunction|PlatformWobling))))

(event Custom|PlatformFalling
  (bind _platformcurrentmovement (Variables|Default|GetPlatformCurrentMovement))
  ;[0.15 0.15 0.15 0.5] Platform Falling
  (bind _floattrack (Timeline|TL_PlatformFalling Play)
    (:Update
      (Transformation|SetRelativeLocation (Variables|Default|GetSM_PlatformFalling) (Math|Vector|Lerp(Vector) _platformcurrentmovement (+ _platformcurrentmovement (Variables|Default|GetPlatformFallingLocation)) _floattrack) false false))
    (:Finished
      (if (Variables|Default|GetIs%20Platform%20Falling)
        (Utilities|FlowControl|Delay (Variables|Default|GetFalling%20Delay))
        (Utilities|String|Reverse (Variables|Default|GetTL_PlatformFalling))
        (Transformation|SetRelativeRotation (Variables|Default|GetSM_PlatformFalling) "0, 0, 0" false false)
        (Variables|Default|SetIs%20Platform%20Falling false)
        (else
          (Audio|Components|Audio|Play (Variables|Default|GetTL_PlatformMovement)))))))

(event Custom|PlatformWobling
  (bind _wobbling_intensity (Variables|Default|GetWobbling%20Intensity))
  (bind _floattrack (Timeline|TL_PlatformWobbling PlayFromStart)
    (:Update
      (Transformation|SetRelativeRotation (Variables|Default|GetSM_PlatformFalling) (Math|Rotator|Lerp(Rotator) (Math|Rotator|MakeRotator 0.0 (Math|Float|Clamp(Float) (* _wobbling_intensity -1.0) -5.0 0.0) 0.0) (Math|Rotator|MakeRotator 0.0 (Math|Float|Clamp(Float) (+ _wobbling_intensity (.pitch (Variables|Default|GetPlatform%20Current%20Rotation))) 0.0 5.0) 0.0) _floattrack) false false))
    (:Finished
      (Utilities|FlowControl|Delay 0.5)
      (Variables|Default|SetIs%20Platform%20Falling true)
      (CallFunction|PlatformFalling))))

(event EventBeginPlay
  (bind _tl_platformmovement (Variables|Default|GetTL_PlatformMovement))
  ;[0.15 0.15 0.15 0.5] Play and Set Speed
  (Audio|Components|Audio|Play _tl_platformmovement)
  (Components|Timeline|SetPlayRate _tl_platformmovement (Variables|Default|GetPlatformSpeed)))

(event Collision|EventActorBeginOverlap
  (params (OtherActor :type Actor%20Object%20Reference)))

(event EventTick
  (params (DeltaSeconds :type Float%20%28single-precision%29)))

(fn ConstructionScript)