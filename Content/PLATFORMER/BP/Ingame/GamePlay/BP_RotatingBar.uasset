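; BP_RotatingBar is a platformer obstacle that spins at a configurable speed and bounces the player character on contact.
; BeginPlay sets the RotatingMovement rate from RotatingSpeed.
; On hit, it mirrors the character's last velocity by the hit normal and scales it by a full or base bounce factor.
; It launches the character with that velocity, clamped by GameInfo limits and never downward, then plays a bounce sound.
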(event Collision|EventHit
  (params (MyComp :type Primitive%20Component%20Object%20Reference) (Other :type Actor%20Object%20Reference) (OtherComp :type Primitive%20Component%20Object%20Reference) (bSelfMoved :type Boolean) (HitLocation :type Vector :default "0, 0, 0") (HitNormal :type Vector :default "0, 0, 0") (NormalImpulse :type Vector :default "0, 0, 0") (Hit :type Hit%20Result%20Structure%20%28by%20ref%29))
  (bind _gameinfo (Variables|Default|GetGameInfo))
  (bind _gameinfo_2 (Variables|Default|GetGameInfo))
  (bind _bounce_xy_max_clamp (Variables|/Game/PLATFORMER/DATA/PDA_GameInfo.PDA_GameInfo_C|GetBounce%20XY%20Max%20Clamp _gameinfo_2))
  (bind _returnvalue (* _bounce_xy_max_clamp -1.0))
  ;[0.15 0.15 0.15 0.5] Bounce
  ;;[0.15 0.15 0.15 0.5] Get Last update Velocity
  (bind _asbp_third_person_character (Utilities|Casting|CastToBP_ThirdPersonCharacter Other))
  (Character|LaunchCharacter _asbp_third_person_character (Math|Vector|MakeVector (Math|Float|Clamp(Float) (.x (* (Math|Vector|MirrorVectorbyNormal (Pawn|Components|CharacterMovement|GetLastUpdateVelocity (Variables|/Script/Engine.Character|GetCharacterMovement _asbp_third_person_character)) HitNormal) (Math|Float|SelectFloat (Variables|/Game/PLATFORMER/DATA/PDA_GameInfo.PDA_GameInfo_C|GetFull%20Bounce%20Velocity _gameinfo) (Variables|/Game/PLATFORMER/DATA/PDA_GameInfo.PDA_GameInfo_C|GetBase%20Bounce%20Velocity _gameinfo) (Variables|Default|GetFull%20Bounce)))) _returnvalue _bounce_xy_max_clamp) (Math|Float|Clamp(Float) (.y (* (Math|Vector|MirrorVectorbyNormal (Pawn|Components|CharacterMovement|GetLastUpdateVelocity (Variables|/Script/Engine.Character|GetCharacterMovement _asbp_third_person_character)) HitNormal) (Math|Float|SelectFloat (Variables|/Game/PLATFORMER/DATA/PDA_GameInfo.PDA_GameInfo_C|GetFull%20Bounce%20Velocity _gameinfo) (Variables|/Game/PLATFORMER/DATA/PDA_GameInfo.PDA_GameInfo_C|GetBase%20Bounce%20Velocity _gameinfo) (Variables|Default|GetFull%20Bounce)))) _returnvalue _bounce_xy_max_clamp) (Math|Float|Clamp(Float) (.z (* (Math|Vector|MirrorVectorbyNormal (Pawn|Components|CharacterMovement|GetLastUpdateVelocity (Variables|/Script/Engine.Character|GetCharacterMovement _asbp_third_person_character)) HitNormal) (Math|Float|SelectFloat (Variables|/Game/PLATFORMER/DATA/PDA_GameInfo.PDA_GameInfo_C|GetFull%20Bounce%20Velocity _gameinfo) (Variables|/Game/PLATFORMER/DATA/PDA_GameInfo.PDA_GameInfo_C|GetBase%20Bounce%20Velocity _gameinfo) (Variables|Default|GetFull%20Bounce)))) 0.0 (Variables|/Game/PLATFORMER/DATA/PDA_GameInfo.PDA_GameInfo_C|GetBounce%20Z%20Max%20Clamp _gameinfo_2))) false false)
  (Audio|PlaySound2D (Variables|/Game/PLATFORMER/DATA/PDA_GameInfo.PDA_GameInfo_C|GetBounceSFX (Variables|Default|GetGameInfo)) 1.0 1.0 0.0 0 0))

(event EventBeginPlay
  ;[0.15 0.15 0.15 0.5] Rotating
  (Variables|/Script/Engine.RotatingMovementComponent|SetRotationRate (Variables|Default|GetRotatingMovement) (Math|Rotator|MakeRotator 0.0 0.0 (Variables|Default|GetRotating%20Speed))))

(fn ConstructionScript)