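; BP_Trap is a platformer trap actor that damages the player character on contact.
; When its TB_Trap component is overlapped by player 0's BP_ThirdPersonCharacter, it applies damage to that character.
; The InstantKill flag selects between the full and base damage values from GameInfos.
; The construction script is empty, and its SetStaticMesh node is never run.
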(event OnComponentBeginOverlap(TB_Trap)
  (params (OverlappedComponent :type Primitive%20Component%20Object%20Reference) (OtherActor :type Actor%20Object%20Reference) (OtherComp :type Primitive%20Component%20Object%20Reference) (OtherBodyIndex :type Integer) (bFromSweep :type Boolean) (SweepResult :type Hit%20Result%20Structure%20%28by%20ref%29))
  (bind _game_infos (Variables|Default|GetGame%20Infos))
  (bind _asbp_third_person_character (Utilities|Casting|CastToBP_ThirdPersonCharacter (Game|GetPlayerCharacter 0)))
  (if (== _asbp_third_person_character OtherActor)
    (Game|Damage|ApplyDamage _asbp_third_person_character (Math|Float|SelectFloat (Variables|/Game/PLATFORMER/DATA/PDA_GameInfo.PDA_GameInfo_C|GetFull%20Damage _game_infos) (Variables|/Game/PLATFORMER/DATA/PDA_GameInfo.PDA_GameInfo_C|GetBase%20Damage _game_infos) (Variables|Default|GetInstant%20Kill)) 0 0)))

(event EventBeginPlay)

(event Collision|EventActorBeginOverlap
  (params (OtherActor :type Actor%20Object%20Reference)))

(event EventTick
  (params (DeltaSeconds :type Float%20%28single-precision%29)))

(fn ConstructionScript)