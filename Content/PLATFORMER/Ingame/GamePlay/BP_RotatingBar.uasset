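; BP_RotatingBar is a platformer obstacle that spins and knocks the player character away on contact.
; On BeginPlay, its RotatingMovement component takes its rate from RotatingSpeed.
; On hit, it mirrors the character's last movement velocity about the hit normal, clamps each axis with only slight upward lift allowed, scales it by BounceVelocity and launches the character, overriding horizontal velocity only.
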(event Collision|EventHit
  (params (MyComp :type Primitive%20Component%20Object%20Reference) (Other :type Actor%20Object%20Reference) (OtherComp :type Primitive%20Component%20Object%20Reference) (bSelfMoved :type Boolean) (HitLocation :type Vector :default "0, 0, 0") (HitNormal :type Vector :default "0, 0, 0") (NormalImpulse :type Vector :default "0, 0, 0") (Hit :type Hit%20Result%20Structure%20%28by%20ref%29))
  ;[0.15 0.15 0.15 0.5] Bounce
  ;;[0.15 0.15 0.15 0.5] Get Last update Velocity
  (bind _asbp_third_person_character (Utilities|Casting|CastToBP_ThirdPersonCharacter Other))
  ;;[0.15 0.15 0.15 0.5] Add Force
  (Character|LaunchCharacter _asbp_third_person_character (* (Math|Vector|MakeVector (Math|Float|Clamp(Float) (.x (Math|Vector|MirrorVectorbyNormal (Pawn|Components|CharacterMovement|GetLastUpdateVelocity (Variables|/Script/Engine.Character|GetCharacterMovement _asbp_third_person_character)) HitNormal)) -5e+02 5e+02) (Math|Float|Clamp(Float) (.y (Math|Vector|MirrorVectorbyNormal (Pawn|Components|CharacterMovement|GetLastUpdateVelocity (Variables|/Script/Engine.Character|GetCharacterMovement _asbp_third_person_character)) HitNormal)) -5e+02 5e+02) (Math|Float|Clamp(Float) (.z (Math|Vector|MirrorVectorbyNormal (Pawn|Components|CharacterMovement|GetLastUpdateVelocity (Variables|/Script/Engine.Character|GetCharacterMovement _asbp_third_person_character)) HitNormal)) 0.0 5e+01)) (Variables|Default|GetBounce%20Velocity)) true false))

(event EventBeginPlay
  ;[0.15 0.15 0.15 0.5] Rotating
  (Variables|/Script/Engine.RotatingMovementComponent|SetRotationRate (Variables|Default|GetRotatingMovement) (Math|Rotator|MakeRotator 0.0 0.0 (Variables|Default|GetRotating%20Speed))))

(fn ConstructionScript)