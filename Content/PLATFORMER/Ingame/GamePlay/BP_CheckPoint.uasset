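; BP_CheckPoint is a checkpoint actor for the platformer mode, with a visible mesh and a box trigger.
; When the third-person character overlaps the box, it stores itself as LastCheckPoint on GM_Platformer and hides its mesh.
; The construction script applies the configurable static mesh and trigger box size to each placed instance.
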(event OnComponentBeginOverlap(TB_Checkpoint)
  (params (OverlappedComponent :type Primitive%20Component%20Object%20Reference) (OtherActor :type Actor%20Object%20Reference) (OtherComp :type Primitive%20Component%20Object%20Reference) (OtherBodyIndex :type Integer) (bFromSweep :type Boolean) (SweepResult :type Hit%20Result%20Structure%20%28by%20ref%29))
  (Utilities|Casting|CastToBP_ThirdPersonCharacter OtherActor)
  (bind _asgm_platformer (Utilities|Casting|CastToGM_Platformer (Game|GetGameMode)))
  (Variables|/Game/PLATFORMER/Ingame/GM/GM_Platformer.GM_Platformer_C|SetLastCheckPoint _asgm_platformer self)
  (Rendering|SetVisibility (Variables|Default|GetSM_CheckPoint) false false))

(fn ConstructionScript
  (Components|StaticMesh|SetStaticMesh (Variables|Default|GetSM_CheckPoint) (Variables|Default|GetStaticMesh))
  (Components|Box|SetBoxExtent (Variables|Default|GetTB_Checkpoint) (Variables|Default|GetTrigger%20Box%20Size) true))