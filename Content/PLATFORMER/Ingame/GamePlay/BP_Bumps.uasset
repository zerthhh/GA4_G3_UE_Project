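; BP_Bumps is a moving bumper that bounces the player character away on hit.
; On BeginPlay it starts a timeline at MovementSpeed play rate, which lerps the bump mesh from its relative origin toward BumpEndLocation.
; On hit, it mirrors the character's last velocity by the hit normal, scales it by base or full bounce values from GameInfos, then launches the character.
; Launch velocity is clamped per axis, with Z never negative.
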(event EventBeginPlay
  (bind _tl_bumpmovement (Variables|Default|GetTL_BumpMovement))
  ;[0.15 0.15 0.15 0.5] Play and Set Speed
  (Audio|Components|Audio|Play _tl_bumpmovement)
  (Components|Timeline|SetPlayRate _tl_bumpmovement (Variables|Default|GetMovementSpeed)))

(event Collision|EventHit
  (params (MyComp :type Primitive%20Component%20Object%20Reference) (Other :type Actor%20Object%20Reference) (OtherComp :type Primitive%20Component%20Object%20Reference) (bSelfMoved :type Boolean) (HitLocation :type Vector :default "0, 0, 0") (HitNormal :type Vector :default "0, 0, 0") (NormalImpulse :type Vector :default "0, 0, 0") (Hit :type Hit%20Result%20Structure%20%28by%20ref%29))
  (bind _game_infos (Variables|Default|GetGame%20Infos))
  (bind _game_infos_2 (Variables|Default|GetGame%20Infos))
  (bind _bounce_xy_max_clamp (Variables|/Game/PLATFORMER/DATA/PDA_GameInfo.PDA_GameInfo_C|GetBounce%20XY%20Max%20Clamp _game_infos_2))
  (bind _returnvalue (* _bounce_xy_max_clamp -1.0))
  ;[0.15 0.15 0.15 0.5] Bounce
  ;;[0.15 0.15 0.15 0.5] Get Last update Velocity
  (bind _asbp_third_person_character (Utilities|Casting|CastToBP_ThirdPersonCharacter Other))
  (Character|LaunchCharacter _asbp_third_person_character (Math|Vector|MakeVector (Math|Float|Clamp(Float) (.x (* (Math|Vector|MirrorVectorbyNormal (Pawn|Components|CharacterMovement|GetLastUpdateVelocity (Variables|/Script/Engine.Character|GetCharacterMovement _asbp_third_person_character)) HitNormal) (Math|Float|SelectFloat (Variables|/Game/PLATFORMER/DATA/PDA_GameInfo.PDA_GameInfo_C|GetFull%20Bounce%20Velocity _game_infos) (Variables|/Game/PLATFORMER/DATA/PDA_GameInfo.PDA_GameInfo_C|GetBase%20Bounce%20Velocity _game_infos) (Variables|Default|GetFull%20Bounce)))) _returnvalue _bounce_xy_max_clamp) (Math|Float|Clamp(Float) (.y (* (Math|Vector|MirrorVectorbyNormal (Pawn|Components|CharacterMovement|GetLastUpdateVelocity (Variables|/Script/Engine.Character|GetCharacterMovement _asbp_third_person_character)) HitNormal) (Math|Float|SelectFloat (Variables|/Game/PLATFORMER/DATA/PDA_GameInfo.PDA_GameInfo_C|GetFull%20Bounce%20Velocity _game_infos) (Variables|/Game/PLATFORMER/DATA/PDA_GameInfo.PDA_GameInfo_C|GetBase%20Bounce%20Velocity _game_infos) (Variables|Default|GetFull%20Bounce)))) _returnvalue _bounce_xy_max_clamp) (Math|Float|Clamp(Float) (.z (* (Math|Vector|MirrorVectorbyNormal (Pawn|Components|CharacterMovement|GetLastUpdateVelocity (Variables|/Script/Engine.Character|GetCharacterMovement _asbp_third_person_character)) HitNormal) (Math|Float|SelectFloat (Variables|/Game/PLATFORMER/DATA/PDA_GameInfo.PDA_GameInfo_C|GetFull%20Bounce%20Velocity _game_infos) (Variables|/Game/PLATFORMER/DATA/PDA_GameInfo.PDA_GameInfo_C|GetBase%20Bounce%20Velocity _game_infos) (Variables|Default|GetFull%20Bounce)))) 0.0 (Variables|/Game/PLATFORMER/DATA/PDA_GameInfo.PDA_GameInfo_C|GetBounce%20Z%20Max%20Clamp _game_infos_2))) false false))

(event EventTick
  (params (DeltaSeconds :type Float%20%28single-precision%29)))

(event Collision|EventActorBeginOverlap
  (params (OtherActor :type Actor%20Object%20Reference)))

(fn ConstructionScript)