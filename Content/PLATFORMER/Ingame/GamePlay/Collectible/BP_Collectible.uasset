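; BP_Collectible is a configurable platformer pickup that grants healing and score to whoever touches it.
; Its construction script applies the chosen static mesh to the SMCollectible component.
; When the TB_Collectible trigger overlaps an actor implementing BPI_Collectible, it sends that actor a PickupMessage with the GameInfo heal and score values, plays the GameInfo sound, and destroys itself.
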(event OnComponentBeginOverlap(TB_Collectible)
  (params (OverlappedComponent :type Primitive%20Component%20Object%20Reference) (OtherActor :type Actor%20Object%20Reference) (OtherComp :type Primitive%20Component%20Object%20Reference) (OtherBodyIndex :type Integer) (bFromSweep :type Boolean) (SweepResult :type Hit%20Result%20Structure%20%28by%20ref%29))
  (bind _game_info (Variables|Default|GetGame%20Info))
  (if (Utilities|DoesObjectImplementInterface OtherActor "/Game/PLATFORMER/Ingame/GamePlay/Collectible/BPI_Collectible.BPI_Collectible_C")
    (Class|BPICollectible|Pickup(Message) OtherActor (Variables|/Game/PLATFORMER/DATA/PDA_GameInfo.PDA_GameInfo_C|GetHeal%20Value _game_info) (Variables|/Game/PLATFORMER/DATA/PDA_GameInfo.PDA_GameInfo_C|GetScore%20Value _game_info))
    (Audio|PlaySound2D (Variables|/Game/PLATFORMER/DATA/PDA_GameInfo.PDA_GameInfo_C|GetCollectibleSFX (Variables|Default|GetGame%20Info)) 1.0 1.0 0.0 0 0)
    (Actor|DestroyActor)))

(event EventBeginPlay)

(event Collision|EventActorBeginOverlap
  (params (OtherActor :type Actor%20Object%20Reference)))

(event EventTick
  (params (DeltaSeconds :type Float%20%28single-precision%29)))

(fn ConstructionScript
  (Components|StaticMesh|SetStaticMesh (Variables|Default|GetSM_Collectible) (Variables|Default|GetStatic%20Mesh)))